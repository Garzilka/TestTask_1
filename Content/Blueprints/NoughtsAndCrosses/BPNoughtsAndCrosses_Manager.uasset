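; Manager for the noughts and crosses game that shows the end-of-game result screen.
; Its CreateWidget event maps a result type to win, lose or no-winner text on a PostGameStatistics widget, treating unknown types as a loss.
; An InterfaceRef validity check prevents a second screen while one exists.
; After creating the widget, it shows the mouse cursor and disables player controller input.
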(event `self.CreateWidget`
  (params (Type :type Integer))
  (bind _returnvalue (`GameplayStatics.GetPlayerController` 0))
  (`self.InterfaceRef`
    (:`then`)
    (:`else`
      (switch `int` Type
        (:`Default`
          (bind _returnvalue_2 (`|CreateWidget` "/Game/Blueprints/UI/Task_2/PostGameStatistics.PostGameStatistics_C" :!label _label))
          (set `self.InterfaceRef` _returnvalue_2)
          (`TextBlock.SetText` (`/Game/Blueprints/UI/Task_2/PostGameStatistics.Tex` _returnvalue_2) "You Lose :(")
          (`UserWidget.AddToViewport` _returnvalue_2 0))
        (:`0`
          (bind _returnvalue_3 (`|CreateWidget` "/Game/Blueprints/UI/Task_2/PostGameStatistics.PostGameStatistics_C"))
          (set `self.InterfaceRef` _returnvalue_3)
          (`TextBlock.SetText` (`/Game/Blueprints/UI/Task_2/PostGameStatistics.Tex` _returnvalue_3) "no winning tactics")
          (`UserWidget.AddToViewport` _returnvalue_3 0))
        (:`1`
          (bind _returnvalue_4 (`|CreateWidget` "/Game/Blueprints/UI/Task_2/PostGameStatistics.PostGameStatistics_C"))
          (set `self.InterfaceRef` _returnvalue_4)
          (`TextBlock.SetText` (`/Game/Blueprints/UI/Task_2/PostGameStatistics.Tex` _returnvalue_4) "You Win :)")
          (`UserWidget.AddToViewport` _returnvalue_4 0))
        (:`2`
          (goto _label)))
      (set `PlayerController.bShowMouseCursor` true _returnvalue)
      (`self.DisableInput` _returnvalue _returnvalue))))

(fn `UserConstructionScript`)